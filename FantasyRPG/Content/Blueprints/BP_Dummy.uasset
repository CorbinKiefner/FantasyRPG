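; BP_Dummy is a target character that reacts to damage and can be stealth-assassinated from behind.
; The AssassinationRadius overlap toggles a prompt widget for the third-person player.
; Damage plays a random hit montage and launches the dummy along the player's facing with some lift.
; StealthBackAssassination plays the victim's paired montage, returns alignment location and rotation for the attacker, and triggers delayed death sound and ragdoll with component cleanup.
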(event OnComponentBeginOverlap(AssassinationRadius)
  (params (OverlappedComponent :type Primitive%20Component%20Object%20Reference) (OtherActor :type Actor%20Object%20Reference) (OtherComp :type Primitive%20Component%20Object%20Reference) (OtherBodyIndex :type Integer) (bFromSweep :type Boolean) (SweepResult :type Hit%20Result%20Structure%20%28by%20ref%29))
  ;[1 1 1] Assassinate Widget
  (Utilities|Casting|CastToBP_ThirdPersonCharacter OtherActor)
  (Rendering|SetVisibility (Variables|Default|GetAssassinate%20Widget) true false))

(event OnComponentEndOverlap(AssassinationRadius)
  (params (OverlappedComponent :type Primitive%20Component%20Object%20Reference) (OtherActor :type Actor%20Object%20Reference) (OtherComp :type Primitive%20Component%20Object%20Reference) (OtherBodyIndex :type Integer))
  ;[1 1 1] Assassinate Widget
  (Utilities|Casting|CastToBP_ThirdPersonCharacter OtherActor)
  (Rendering|SetVisibility (Variables|Default|GetAssassinate%20Widget) false false))

(event Custom|Ragdoll
  ;[1 1 1] Ragdoll
  (Utilities|FlowControl|Sequence
    (:then_0
      (Utilities|FlowControl|Delay 2.1)
      (Physics|SetSimulatePhysics (Variables|Character|GetMesh) true)
      (Components|DestroyComponent (Variables|Collision|GetCapsuleComponent))
      (Components|DestroyComponent (Variables|Default|GetAssassination%20Radius))
      (Components|DestroyComponent (Variables|Default|GetAssassin%20REF)))
    (:then_1
      (Utilities|FlowControl|Delay 1.75)
      (Audio|PlaySoundatLocation "/Game/Audio/HitGrunts/SC_Death.SC_Death" (Transformation|GetActorLocation) "0, 0, 0" 1.0 1.0 0.0 0 0 0 0))))

(event Game|Damage|EventAnyDamage
  (params (Damage :type Float%20%28single-precision%29) (DamageType :type Damage%20Type%20Object%20Reference) (InstigatedBy :type Controller%20Object%20Reference) (DamageCauser :type Actor%20Object%20Reference))
  (bind _hitanims (Variables|Default|GethitAnims))
  (Animation|PlayAnimMontage (Utilities|Array|Get(acopy) _hitanims (Math|Random|RandomIntegerinRange 0 (- (Utilities|Array|Length _hitanims) 1))) 1.0 "None")
  (bind _asbp_third_person_character (Utilities|Casting|CastToBP_ThirdPersonCharacter (Game|GetPlayerCharacter 0)))
  (Character|LaunchCharacter (Math|Vector|MakeVector (.x (* (Math|Vector|GetForwardVector (Transformation|GetActorRotation _asbp_third_person_character)) 3e+02)) (.y (* (Math|Vector|GetForwardVector (Transformation|GetActorRotation _asbp_third_person_character)) 3e+02)) 2e+02) false false))

(fn ConstructionScript)

(fn StealthBackAssassination
  (Animation|PlayAnimMontage "/Game/Characters/RPG_Character/Animations/Assassinations/Paired_Knife_Stealth_KidneyAndNeck_Vic_Montage.Paired_Knife_Stealth_KidneyAndNeck_Vic_Montage" 1.0 "None")
  (CallFunction|Ragdoll)
  (Rendering|SetVisibility (Variables|Default|GetAssassinate%20Widget) false false)
  (return (Transformation|GetWorldLocation (Variables|Default|GetAssassin%20REF)) (Transformation|GetActorRotation)))